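; Game mode Blueprint that sets up a two-team agent simulation, Red versus Blue, when play begins.
; It finds the Red and Blue leader agents in the level and registers each team with its leader component, name and color, then marks the teams as mutual enemies.
; It then registers every follower agent in the level as a member of the team given by that agent's own TeamID.
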(event EventBeginPlay
  (bind _returnvalue (Actor|GetActorOfClass "/Game/Game/Blueprints/Actor/Characters/BP_RedLeaderAgent.BP_RedLeaderAgent_C"))
  (bind _returnvalue_2 (Actor|GetActorOfClass "/Game/Game/Blueprints/Actor/Characters/BP_BlueLeaderAgent.BP_BlueLeaderAgent_C"))
  (Class|SimulationManagerGameMode|RegisterTeam 0 (Variables|/Script/GameAI_Project.LeaderCharacter|GetTeamLeaderComponent _returnvalue) "Red" "(R=1.000000,G=0.000000,B=0.000000,A=1.000000)")
  (Class|SimulationManagerGameMode|RegisterTeam 1 (Variables|/Script/GameAI_Project.LeaderCharacter|GetTeamLeaderComponent _returnvalue_2) "Blue" "(R=0.000000,G=0.000000,B=1.000000,A=1.000000)")
  (Class|SimulationManagerGameMode|SetMutualEnemies 0 1)
  (bind _outactors (Actor|GetAllActorsOfClass "/Game/Game/Blueprints/Actor/Characters/BP_FollowerAgent.BP_FollowerAgent_C"))
  (for _array_element _outactors
    (Class|SimulationManagerGameMode|RegisterTeamMember (Variables|/Game/Game/Blueprints/Actor/Characters/BP_FollowerAgent.BP_FollowerAgent_C|GetTeamID _array_element) _array_element)))

(event EventTick
  (params (DeltaSeconds :type Float%20%28single-precision%29)))

(fn ConstructionScript)