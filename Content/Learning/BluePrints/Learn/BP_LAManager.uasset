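; BP_LAManager is a Learning Agents manager actor that sets up a neural-network policy for the BP_AAgent actors in the level.
; BeginPlay gathers the agents, makes them tick after itself, and builds Interactor, Policy and Critic, reinitializing networks unless RunInference is set.
; With RunInference on, the first agent's episode resets and Tick runs policy inference.
; Training is unfinished: no Trainer is created and RunTraining is never reached.
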(event EventBeginPlay
  (bind _runinference (Variables|Default|GetRunInference))
  (bind _returnvalue (not _runinference))
  (Utilities|FlowControl|Sequence
    (:then_0
      (bind _outactors (Actor|GetAllActorsOfClass "/Game/Learning/BluePrints/BP_AAgent.BP_AAgent_C"))
      (bind _output_get (Variables|Default|SetAgents _outactors))
      (Actor|Tick|AddTickPrerequisiteActor _output_get self))
    (:then_1
      (bind _returnvalue_2 (Class|LearningAgentsInteractor|MakeInteractor (Variables|Default|GetLearningAgentsManager) "/Game/Learning/BluePrints/Learn/BP_LAInteractor.BP_LAInteractor_C" "Interactor" :!label _label))
      (Variables|Default|SetInteractor _returnvalue_2))
    (:then_2
      (goto _label))
    (:then_3
      (bind _returnvalue_3 (Class|LearningAgentsPolicy|MakePolicy (Variables|Default|GetLearningAgentsManager) (Variables|Default|GetInteractor) "/Script/LearningAgents.LearningAgentsPolicy" "Policy" "/Game/Learning/BluePrints/Learn/DA_LANeuralNetworkEncoder.DA_LANeuralNetworkEncoder" "/Game/Learning/BluePrints/Learn/DA_LANeuralNetworkPolicy.DA_LANeuralNetworkPolicy" "/Game/Learning/BluePrints/Learn/DA_LANeuralNetworkDecoder.DA_LANeuralNetworkDecoder" _returnvalue _returnvalue _returnvalue (Variables|Default|GetPolicy%20Settings) 1234))
      (Variables|Default|SetPolicy _returnvalue_3))
    (:then_4
      (bind _returnvalue_4 (Class|LearningAgentsCritic|MakeCritic (Variables|Default|GetLearningAgentsManager) (Variables|Default|GetInteractor) (Variables|Default|GetPolicy) "/Script/LearningAgents.LearningAgentsCritic" "Critic" "/Game/Learning/BluePrints/Learn/DA_LANeuralNetworkCritic.DA_LANeuralNetworkCritic" (not (Variables|Default|GetRunInference)) (Variables|Default|GetCritic%20Settings) 1234))
      (Variables|Default|SetCritic _returnvalue_4))
    (:then_6
      (if (Variables|Default|GetRunInference)
        (Default|ResetEpisode (Utilities|Array|Get(acopy) (Variables|Default|GetAgents)))))))

(event Collision|EventActorBeginOverlap
  (params (OtherActor :type Actor%20Object%20Reference)))

(event EventTick
  (params (DeltaSeconds :type Float%20%28single-precision%29))
  (if (Variables|Default|GetRunInference)
    (Class|LearningAgentsPolicy|RunInference (Variables|Default|GetPolicy) 3.0)
    (else
      (Utilities|IsValid 0))))

(fn ConstructionScript)